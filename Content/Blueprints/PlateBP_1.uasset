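; PlateBP_1 is a plate actor whose metal plate component follows a separate PivotBase component.
; The construction script snaps PivotBase to PlateMetal's world transform, then attaches CollisionCorner1 to the pivot, keeping its world position.
; Every Tick, PlateMetal teleports to the pivot's world location and rotation, so the plate mirrors any movement of the pivot.
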(event `self.ReceiveTick`
  (params (DeltaSeconds :type "Float (single-precision)"))
  (bind _pivotbase (`self.PivotBase`))
  (`SceneComponent.K2_SetWorldLocationAndRotation` (`self.PlateMetal`) (`SceneComponent.K2_GetComponentLocation` _pivotbase) (`KismetMathLibrary.MakeRotator` (.roll (`SceneComponent.K2_GetComponentRotation` _pivotbase)) (.pitch (`SceneComponent.K2_GetComponentRotation` _pivotbase)) (.yaw (`SceneComponent.K2_GetComponentRotation` _pivotbase))) false true))

(fn `UserConstructionScript`
  (bind _platemetal (`self.PlateMetal`))
  (`SceneComponent.K2_SetWorldLocationAndRotation` (`self.PivotBase`) (`SceneComponent.K2_GetComponentLocation` _platemetal) (`SceneComponent.K2_GetComponentRotation` _platemetal) false true)
  (`SceneComponent.K2_AttachTo` (`self.CollisionCorner_1`) (`self.PivotBase`) "None" "KeepWorldPosition" true))