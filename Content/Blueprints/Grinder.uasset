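; Grinder actor with two static meshes that spin continuously in opposite directions.
; Tick adds local yaw from Speed to each mesh, getting the reverse spin through a rotator delta against twice Speed, without delta-time scaling, so rotation depends on frame rate.
; The construction script places the second mesh at a fixed X offset with Openlength as its Z, setting the gap.
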(event `self.ReceiveBeginPlay`)

(event `self.ReceiveActorBeginOverlap`
  (params (OtherActor :type "Actor Object Reference")))

(event `self.ReceiveTick`
  (params (DeltaSeconds :type "Float (single-precision)"))
  (bind _speed (`self.Speed`))
  (bind _returnvalue (`KismetMathLibrary.MakeRotator` 0.0 0.0 _speed))
  (`SceneComponent.K2_AddLocalRotation` (`self.StaticMesh`) (`KismetMathLibrary.NormalizedDeltaRotator` _returnvalue (`KismetMathLibrary.MakeRotator` 0.0 0.0 (* _speed 2.0))) false false)
  (`SceneComponent.K2_AddLocalRotation` (`self.StaticMesh1`) _returnvalue false false))

(fn `UserConstructionScript`
  (`SceneComponent.K2_SetRelativeLocation` (`self.StaticMesh1`) (`KismetMathLibrary.MakeVector` -150.0 0.0 (`self.Openlength`)) false false))