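; ShootBlock is the input controller for a car-physics sandbox, adding brick guns, slow motion and scene reset.
; Tick copies gas, toggled brake and reverse input to every BP_Car, and applies off-center force to flip them.
; A Delay on Tick paces held-fire bricks; alternate fire launches large ones.
; Reset respawns cars with their paint, destroys boxes, and restores props, destructibles and bricks from transforms cached at BeginPlay.
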(event `Key|Tab`
  (params (Key :type "Key Structure" :default "AnyKey"))
  ;[1 1 1] Slow Motion
  (:`Pressed`
    (`/Engine/EditorBlueprintResources/StandardMacros.FlipFlop`
      (:`A`
        (`GameplayStatics.SetGlobalTimeDilation` 1.0))
      (:`B`
        (`GameplayStatics.SetGlobalTimeDilation` 0.1)))))

(event `self.ReceiveTick`
  (params (DeltaSeconds :type "Float (single-precision)"))
  (bind _returnvalue (`GameplayStatics.GetPlayerController` 0))
  (bind _returnvalue_2 (`self.GetActorForwardVector` (`GameplayStatics.GetPlayerController` 0)))
  (`|ExecutionSequence`
    (:`then_0`
      (`|ExecutionSequence`
        (:`then_0`
          ;[1 1 1] Gas
          (bind _outactors (`GameplayStatics.GetAllActorsOfClass` "/Game/Blueprints/BP_Car.BP_Car_C"))
          (for _index (range (`KismetArrayLibrary.Array_Length` _outactors))
            (set `/Game/Blueprints/BP_Car.Gas` (`self.F Down`) (`KismetArrayLibrary.Array_Get` _outactors _index))))
        (:`then_1`
          ;[1 1 1] Brake
          (bind _outactors_2 (`GameplayStatics.GetAllActorsOfClass` "/Game/Blueprints/BP_Car.BP_Car_C"))
          (for _index_2 (range (`KismetArrayLibrary.Array_Length` _outactors_2))
            (set `/Game/Blueprints/BP_Car.Brake` (`self.V Down`) (`KismetArrayLibrary.Array_Get` _outactors_2 _index_2))))
        (:`then_2`
          ;[1 1 1] Flip Car
          (if (`self.T Down`)
            (bind _outactors_3 (`GameplayStatics.GetAllActorsOfClass` "/Game/Blueprints/BP_Car.BP_Car_C"))
            (for _index_3 (range (`KismetArrayLibrary.Array_Length` _outactors_3))
              (bind _carbase (`/Game/Blueprints/BP_Car.CARBASE` (`KismetArrayLibrary.Array_Get` _outactors_3 _index_3)))
              (`PrimitiveComponent.AddForceAtLocation` _carbase (* (`KismetMathLibrary.GetUpVector` (struct)) 500000.0) (+ (`SceneComponent.K2_GetComponentLocation` _carbase) (* (`SceneComponent.GetRightVector` _carbase) 300.0)) "None"))))
        (:`then_3`
          ;[1 1 1] Reverse
          (bind _outactors_4 (`GameplayStatics.GetAllActorsOfClass` "/Game/Blueprints/BP_Car.BP_Car_C"))
          (for _array_element _outactors_4
            (set `/Game/Blueprints/BP_Car.Reverse` (or (`PlayerController.IsInputKeyDown` _returnvalue "G") (`PlayerController.IsInputKeyDown` _returnvalue "Gamepad_FaceButton_Right")) _array_element)))))
    (:`then_1`
      ;[1 1 1] Brick Gun
      (if (`self.LeftDown`)
        (`KismetSystemLibrary.Delay` 0.1)
        (bind _returnvalue_3 (`|SpawnActorFromClass` "/Game/Blueprints/BP_Brick.BP_Brick_C" (`KismetMathLibrary.MakeTransform` (+ (* _returnvalue_2 10.0) (.location (`self.GetTransform` (`GameplayStatics.GetPlayerPawn` 0)))) (`KismetMathLibrary.RandomRotator` false) (1.0 1.0 1.0)) "AlwaysSpawn" "OverrideRootScale"))
        (`PrimitiveComponent.SetPhysicsLinearVelocity` (`StaticMeshActor.StaticMeshComponent` _returnvalue_3) (* _returnvalue_2 (* 1000.0 1.0)) false "None")))))

(event `Key|Gamepad_RightTrigger`
  (params (Key :type "Key Structure" :default "AnyKey"))
  ;[1 1 1] Left Mouse Event
  (:`Pressed`
    (set `self.LeftDown` true :!label _label))
  (:`Released`
    (set `self.LeftDown` false :!label _label_2)))

(event `Key|LeftMouseButton` :consume false
  (params (Key :type "Key Structure" :default "AnyKey"))
  ;[1 1 1] Left Mouse Event
  (:`Pressed`
    (goto _label))
  (:`Released`
    (goto _label_2)))

(event `Key|RightMouseButton`
  (params (Key :type "Key Structure" :default "AnyKey"))
  (bind _returnvalue (`self.GetActorForwardVector` (`GameplayStatics.GetPlayerController` 0)))
  ;[1 1 1] Large Brick Gun
  (:`Pressed`
    (bind _returnvalue_2 (`|SpawnActorFromClass` "/Game/Blueprints/BP_Brick.BP_Brick_C" (`KismetMathLibrary.MakeTransform` (+ (* _returnvalue 10.0) (.location (`self.GetTransform` (`GameplayStatics.GetPlayerPawn` 0)))) (`KismetMathLibrary.RandomRotator` false) (3.0 3.0 3.0)) "AlwaysSpawn" "OverrideRootScale" :!label _label_3))
    (`PrimitiveComponent.SetPhysicsLinearVelocity` (`StaticMeshActor.StaticMeshComponent` _returnvalue_2) (* _returnvalue (* 1000.0 1.0)) false "None")))

(event `Key|Gamepad_LeftTrigger`
  (params (Key :type "Key Structure" :default "AnyKey"))
  ;[1 1 1] Large Brick Gun
  (:`Pressed`
    (goto _label_3)))

(event `self.ReceiveBeginPlay`
  ;[1 1 1] Set Reset Location Arrays
  (`|ExecutionSequence`
    (:`then_0`
      (bind _outactors (`GameplayStatics.GetAllActorsOfClass` "/Script/Engine.StaticMeshActor"))
      (for _array_element _outactors
        (`KismetArrayLibrary.Array_Add` (`self.Static Location Array`) (`self.GetTransform` _array_element))))
    (:`then_1`
      (bind _outactors_2 (`GameplayStatics.GetAllActorsOfClass` "/Game/Blueprints/BP_Barrier_Concrete_DM.BP_Barrier_Concrete_DM_C"))
      (for _array_element_2 _outactors_2
        (`KismetArrayLibrary.Array_Add` (`self.Barrier Array`) (`self.GetTransform` _array_element_2))))
    (:`then_2`
      (bind _outactors_3 (`GameplayStatics.GetAllActorsOfClass` "/Game/Blueprints/BP_Wall_400x200_DM.BP_Wall_400x200_DM_C"))
      (for _array_element_3 _outactors_3
        (`KismetArrayLibrary.Array_Add` (`self.DestructibleWall Array`) (`self.GetTransform` _array_element_3))))
    (:`then_3`
      (bind _outactors_4 (`GameplayStatics.GetAllActorsOfClass` "/Game/Blueprints/BP_Brick.BP_Brick_C"))
      (for _array_element_4 _outactors_4
        (`KismetArrayLibrary.Array_Add` (`self.BrickArray`) (`self.GetTransform` _array_element_4))))))

(event `Key|Gamepad_DPad_Up`
  (params (Key :type "Key Structure" :default "AnyKey"))
  ;[1 1 1] Forward Event
  (:`Pressed`
    (set `self.F Down` true :!label _label_4))
  (:`Released`
    (set `self.F Down` false :!label _label_5)))

(event `Key|F`
  (params (Key :type "Key Structure" :default "AnyKey"))
  ;[1 1 1] Forward Event
  (:`Pressed`
    (goto _label_4))
  (:`Released`
    (goto _label_5)))

(event `Key|R`
  (params (Key :type "Key Structure" :default "AnyKey"))
  (bind _temp (`self.Temp`))
  (bind _car_roughenss (`/Game/Blueprints/BP_Car.Car Roughenss` _temp))
  ;[1 1 1] Reset Scene
  (:`Pressed`
    (bind _outactors (`GameplayStatics.GetAllActorsOfClass` "/Game/Blueprints/BP_Box.BP_Box_C" :!label _label_6))
    (`self.K2_DestroyActor` _outactors)
    (`|ExecutionSequence`
      (:`then_0`
        (bind _outactors_2 (`GameplayStatics.GetAllActorsOfClass` "/Game/Blueprints/BP_Car.BP_Car_C"))
        (for _index (range (`KismetArrayLibrary.Array_Length` _outactors_2))
          (bind _output_get (set `self.Temp` (`KismetArrayLibrary.Array_Get` _outactors_2 _index)))
          (bind _returnvalue (`|SpawnActorFromClass` (select `bool` (== (`GameplayStatics.GetObjectClass` _output_get) "/Game/Blueprints/BP_Car_Closed.BP_Car_Closed_C") :`false` "/Game/Blueprints/BP_Car.BP_Car_C" :`true` "/Game/Blueprints/BP_Car_Closed.BP_Car_Closed_C" :!type "Actor Class Reference") (`self.GetTransform` _output_get) "AdjustIfPossibleButAlwaysSpawn" "OverrideRootScale"))
          (bind _asbp_car (cast `/Game/Blueprints/BP_Car` _returnvalue))
          (set `/Game/Blueprints/BP_Car.Car Roughenss` _car_roughenss _asbp_car)
          (bind _output_get_2 (set `/Game/Blueprints/BP_Car.Car Color` (`/Game/Blueprints/BP_Car.Car Color` _temp) _asbp_car))
          (for _array_element (`|MakeArray` (`/Game/Blueprints/BP_Car.Deform_Hood` _asbp_car) (`/Game/Blueprints/BP_Car.Deform_Door_Left` _asbp_car) (`/Game/Blueprints/BP_Car.Deform_Back` _asbp_car) (`/Game/Blueprints/BP_Car.Deform_Door_Left_Back` _asbp_car) (`/Game/Blueprints/BP_Car.Deform_Door_Right` _asbp_car) (`/Game/Blueprints/BP_Car.Deform_Door_Right_Back` _asbp_car) (`/Game/Blueprints/BP_Car.Deform_LeftFend` _asbp_car) (`/Game/Blueprints/BP_Car.Deform_RightFend` _asbp_car) (`/Game/Blueprints/BP_Car.Deform_Top` _asbp_car) (`/Game/Blueprints/BP_Car.Deform_Trunk` _asbp_car))
            (bind _returnvalue_2 (`PrimitiveComponent.CreateDynamicMaterialInstance` _array_element 0 (`PrimitiveComponent.GetMaterial` _array_element 0)))
            (`MaterialInstanceDynamic.SetVectorParameterValue` _returnvalue_2 "Paint Color" _output_get_2)
            (`MaterialInstanceDynamic.SetScalarParameterValue` _returnvalue_2 "Roughness Adjust" _car_roughenss)
            (`MaterialInstanceDynamic.SetScalarParameterValue` _returnvalue_2 "damage" (`/Game/Blueprints/BP_Car.Material Damage` _temp)))
          (`self.K2_DestroyActor` (`self.Temp`))))
      (:`then_1`
        (bind _outactors_3 (`GameplayStatics.GetAllActorsOfClass` "/Script/Engine.StaticMeshActor"))
        (for (_array_element_2 _array_index) _outactors_3
          (if (select `EComponentMobility` (`SceneComponent.Mobility` (`StaticMeshActor.StaticMeshComponent` _array_element_2)) :`Movable` true)
            (`self.K2_SetActorTransform` _array_element_2 (`KismetArrayLibrary.Array_Get` (`self.Static Location Array`) _array_index) false true)
            (`PrimitiveComponent.SetPhysicsLinearVelocity` (`StaticMeshActor.StaticMeshComponent` _array_element_2) (0.0 0.0 0.0) false "None"))))
      (:`then_2`
        (bind _outactors_4 (`GameplayStatics.GetAllActorsOfClass` "/Game/Blueprints/BP_Barrier_Concrete_DM.BP_Barrier_Concrete_DM_C"))
        (for (_array_element_3 _array_index_2) _outactors_4
          (`self.K2_DestroyActor` _array_element_3)
          (bind _returnvalue_3 (`|SpawnActorFromClass` "/Game/Blueprints/BP_Barrier_Concrete_DM.BP_Barrier_Concrete_DM_C" (`KismetArrayLibrary.Array_Get` (`self.Barrier Array`) _array_index_2) "AlwaysSpawn" "OverrideRootScale"))
          (`PrimitiveComponent.SetPhysicsLinearVelocity` (`DestructibleActor.DestructibleComponent` _returnvalue_3) (0.0 0.0 0.0) false "None")))
      (:`then_3`
        (bind _outactors_5 (`GameplayStatics.GetAllActorsOfClass` "/Game/Blueprints/BP_Wall_400x200_DM.BP_Wall_400x200_DM_C"))
        (for (_array_element_4 _array_index_3) _outactors_5
          (`self.K2_DestroyActor` _array_element_4)
          (bind _returnvalue_4 (`|SpawnActorFromClass` "/Game/Blueprints/BP_Wall_400x200_DM.BP_Wall_400x200_DM_C" (`KismetArrayLibrary.Array_Get` (`self.DestructibleWall Array`) _array_index_3) "AlwaysSpawn" "OverrideRootScale"))
          (`PrimitiveComponent.SetPhysicsLinearVelocity` (`DestructibleActor.DestructibleComponent` _returnvalue_4) (0.0 0.0 0.0) false "None")))
      (:`then_4`
        (bind _outactors_6 (`GameplayStatics.GetAllActorsOfClass` "/Game/Blueprints/BP_Brick.BP_Brick_C"))
        (for _array_element_5 _outactors_6
          (`self.K2_DestroyActor` _array_element_5))
        (for _array_element_6 (`self.BrickArray`)
          (bind _returnvalue_5 (`|SpawnActorFromClass` "/Game/Blueprints/BP_Brick.BP_Brick_C" _array_element_6 "AlwaysSpawn" "OverrideRootScale"))
          (`self.SetLifeSpan` _returnvalue_5 0.0))))))

(event `Key|Gamepad_DPad_Left`
  (params (Key :type "Key Structure" :default "AnyKey"))
  ;[1 1 1] Reset Scene
  (:`Pressed`
    (goto _label_6)))

(event `Key|V`
  (params (Key :type "Key Structure" :default "AnyKey"))
  ;[1 1 1] Brake Event
  (:`Pressed`
    (bind _isa (`/Engine/EditorBlueprintResources/StandardMacros.FlipFlop` :!label _label_7)
      (:`A`
        _)
      (:`B`
        _))
    (set `self.V Down` _isa)))

(event `Key|Gamepad_DPad_Down`
  (params (Key :type "Key Structure" :default "AnyKey"))
  ;[1 1 1] Brake Event
  (:`Pressed`
    (goto _label_7)))

(event `Key|T`
  (params (Key :type "Key Structure" :default "AnyKey"))
  ;[1 1 1] Flip Event
  (:`Pressed`
    (set `self.T Down` true))
  (:`Released`
    (set `self.T Down` false)))

(fn `UserConstructionScript`)