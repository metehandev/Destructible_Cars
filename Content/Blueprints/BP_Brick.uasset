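; BP_Brick is a brick actor that sets a limited life span on spawn and plays impact sounds when its mesh is hit.
; Each hit converts the impulse magnitude through a power curve into a clamped strength, which, divided by actor X scale, must pass a threshold to trigger the sound.
; That strength sets the attenuated sound's volume at the impact point, while pitch is randomized and lowered for larger bricks.
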(event `self.ReceiveBeginPlay`
  (`self.SetLifeSpan` (`self.InitialLifeSpan`)))

(event `self.ReceiveActorBeginOverlap`
  (params (OtherActor :type "Actor Object Reference")))

(event `self.ReceiveTick`
  (params (DeltaSeconds :type "Float (single-precision)")))

(event `self.StaticMeshComponent.OnComponentHit`
  (params (OtherActor :type "Actor Object Reference") (OtherComp :type "PrimitiveComponent Object Reference") (NormalImpulse :type "Vector Structure") (Hit :type "HitResult Structure (by ref)"))
  (bind _x (.x (`self.GetActorScale3D`)))
  (bind _returnvalue (`KismetMathLibrary.FClamp` (/ (- (`KismetMathLibrary.MultiplyMultiply_FloatFloat` (`KismetMathLibrary.VSize` NormalImpulse) 0.14) 3.0) 3.0)))
  (if (> (/ _returnvalue _x) 0.3)
    (`GameplayStatics.PlaySoundAtLocation` "/Game/Sounds/Bricksound.Bricksound" (`.ImpactPoint` (`GameplayStatics.BreakHitResult` Hit)) (struct) _returnvalue (/ (`KismetMathLibrary.RandomFloatInRange` 0.5 1.2) (`KismetMathLibrary.FClamp` (/ _x 2.0) 1.0 2.0)) 0.01 "/Game/Sounds/Default_Attenuation.Default_Attenuation")))

(fn `UserConstructionScript`)